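; Shared camera actor for a side-view fighting game that keeps both fighters framed.
; On BeginPlay it waits briefly, then caches Player1 and Player2 from the fighting game mode.
; Each tick it moves to their midpoint in X and Z, keeping its own Y.
; It zooms by scaling field of view with their horizontal X separation, clamped to a fixed range.
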(event EventBeginPlay
  (Utilities|FlowControl|Delay 0.2)
  (bind _asfighting_gamemode (Utilities|Casting|CastTofighting_gamemode (Game|GetGameMode)))
  (Utilities|IsValid (Variables|/Game/Characters/Monk/Blueprint/fighting_gamemode.fighting_gamemode_C|Getplayer1 _asfighting_gamemode)
    (:Is%20Valid
      (Variables|Default|Setplayer1_camera_ref (Variables|/Game/Characters/Monk/Blueprint/fighting_gamemode.fighting_gamemode_C|Getplayer1 _asfighting_gamemode))
      (Utilities|IsValid (Variables|/Game/Characters/Monk/Blueprint/fighting_gamemode.fighting_gamemode_C|Getplayer2 _asfighting_gamemode)
        (:Is%20Valid
          (Variables|Default|Setplayer2_camera_ref (Variables|/Game/Characters/Monk/Blueprint/fighting_gamemode.fighting_gamemode_C|Getplayer2 _asfighting_gamemode)))))))

(event Collision|EventActorBeginOverlap
  (params (OtherActor :type Actor%20Object%20Reference)))

(event EventTick
  (params (DeltaSeconds :type Float%20%28single-precision%29))
  (bind _player1_camera_ref (Variables|Default|Getplayer1_camera_ref))
  (bind _player2_camera_ref (Variables|Default|Getplayer2_camera_ref))
  (bind _returnvalue (Transformation|GetActorLocation _player1_camera_ref))
  (bind _returnvalue_2 (Transformation|GetActorLocation _player2_camera_ref))
  (if (and (Utilities|IsValid _player1_camera_ref) (Utilities|IsValid _player2_camera_ref))
    (Transformation|SetActorLocation (Math|Vector|MakeVector (/ (+ (.x _returnvalue) (.x _returnvalue_2)) 2.0) (.y (Transformation|GetActorLocation)) (/ (+ (.z _returnvalue) (.z _returnvalue_2)) 2.0)) false false)
    (Camera|SetFieldOfView (Variables|CameraActor|GetCameraComponent) (Math|Float|Clamp(Float) (Math|Float|Absolute(Float) (* (- (.x (Transformation|GetActorLocation (Variables|Default|Getplayer1_camera_ref))) (.x (Transformation|GetActorLocation (Variables|Default|Getplayer2_camera_ref)))) 0.1)) 6e+01 9e+01))))

(fn ConstructionScript)