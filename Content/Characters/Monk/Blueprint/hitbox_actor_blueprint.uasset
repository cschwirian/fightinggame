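; Hitbox actor for a two-player fighting game that shows an attack volume and damages the opposing character.
; On spawn it takes an owner, colors its display mesh by type (proximity, strike or hurtbox), then positions and scales that mesh.
; A one-time overlap check then applies damage to whichever player is not the owner, regardless of type.
; Hitstop calls on both players are present but unconnected.
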(event Custom|check_collision
  (bind _returnvalue (Game|GetPlayerCharacter 0))
  (bind _returnvalue_2 (Game|GetPlayerCharacter 1))
  (if (== (Components|GetOwner) (Game|GetPlayerCharacter 0))
    (if (Collision|IsOverlappingActor _returnvalue_2 :!class /Script/Engine.Actor)
      (bind _asplayer_character_blueprint (Utilities|Casting|CastToplayer_character_blueprint _returnvalue_2))
      (Game|Damage|ApplyDamage _asplayer_character_blueprint (Variables|Default|Gethitbox_damage) 0 0))
    (elif (Collision|IsOverlappingActor _returnvalue :!class /Script/Engine.Actor)
      (bind _asplayer_character_blueprint_2 (Utilities|Casting|CastToplayer_character_blueprint _returnvalue))
      (Game|Damage|ApplyDamage _asplayer_character_blueprint_2 (Variables|Default|Gethitbox_damage) 0 0))))

(event Custom|spawn_hitbox
  (params (owner :type Character%20Object%20Reference))
  ;[1 1 1 1 72] spawn_hitbox
  (Actor|SetOwner owner)
  (switch Utilities|FlowControl|Switch|Switchonhitbox_types (Variables|Default|Gethitbox_type)
    (:NewEnumerator0
      (Rendering|Material|SetMaterial (Variables|Default|Gethitbox_display) 0 "/Game/Materials/proximity_hitbox.proximity_hitbox"))
    (:NewEnumerator1
      (Rendering|Material|SetMaterial (Variables|Default|Gethitbox_display) 0 "/Game/Materials/strike_hitbox.strike_hitbox"))
    (:NewEnumerator2
      (Rendering|Material|SetMaterial (Variables|Default|Gethitbox_display) 0 "/Game/Materials/hurtbox_hitbox.hurtbox_hitbox")))
  (Transformation|SetWorldLocation (Variables|Default|Gethitbox_display) (Variables|Default|Gethitbox_location) false false)
  (Transformation|SetWorldScale3D (Variables|Default|Gethitbox_display) (Variables|Default|Gethitbox_scale))
  (Rendering|SetVisibility (Variables|Default|Gethitbox_display) true false)
  (CallFunction|CheckCollision))

(event EventBeginPlay)

(event Collision|EventActorBeginOverlap
  (params (OtherActor :type Actor%20Object%20Reference)))

(event EventTick
  (params (DeltaSeconds :type Float%20%28single-precision%29)))

(fn ConstructionScript)