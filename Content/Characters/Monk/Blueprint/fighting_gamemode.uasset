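; Game mode for a two-player local fighting game that spawns both fighters and shows the HUD.
; On BeginPlay it passes every PlayerStart to SpawnPlayers, which spawns a character at the starts tagged player1 and player2.
; The first is possessed by controller 0 and the second by a newly created local player, and each then loads its controls.
; The HUD widget is created for the first player's controller only.
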(event EventBeginPlay
  (bind _outactors (Actor|GetAllActorsOfClass "/Script/Engine.PlayerStart"))
  (for _array_element _outactors
    (CallFunction|SpawnPlayers _array_element))
  (bind _returnvalue (UserInterface|CreateWidget "/Game/UI/hud.hud_C" (Game|GetPlayerController 0)))
  (UserInterface|Viewport|AddtoViewport _returnvalue 10))

(event EventTick
  (params (DeltaSeconds :type Float%20%28single-precision%29)))

(fn ConstructionScript)

(fn SpawnPlayers
  (params (object :type Actor%20Object%20Reference))
  (bind _asplayer_start (Utilities|Casting|CastToPlayerStart object))
  (if (== (Variables|/Script/Engine.PlayerStart|GetPlayerStartTag _asplayer_start) "player1")
    (bind _returnvalue (Game|SpawnActorfromClass "/Game/Characters/Monk/Blueprint/player_character_blueprint.player_character_blueprint_C" (Transformation|GetActorTransform object) "Undefined" "MultiplyWithRoot" object false 0))
    (bind _output_get (Variables|Default|Setplayer1 _returnvalue))
    (Pawn|Possess (Game|GetPlayerController 0) _output_get)
    (Default|LoadControls _output_get)
    (elif (== (Variables|/Script/Engine.PlayerStart|GetPlayerStartTag _asplayer_start) "player2")
      (bind _returnvalue_2 (Game|SpawnActorfromClass "/Game/Characters/Monk/Blueprint/player_character_blueprint.player_character_blueprint_C" (Transformation|GetActorTransform object) "Undefined" "MultiplyWithRoot" object false 0))
      (bind _output_get_2 (Variables|Default|Setplayer2 _returnvalue_2))
      (bind _returnvalue_3 (Class|GameplayStatics|CreatePlayer -1))
      (Pawn|Possess _returnvalue_3 _output_get_2)
      (Default|LoadControls _output_get_2))))